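; Player-controlled tank Blueprint that handles camera aiming and firing input.
; On BeginPlay it registers its turret and barrel components through reference setters.
; Vertical aim pitches an elevation gimbal by the raw axis value, while horizontal aim yaws the spring arm at a frame-rate-scaled speed.
; The Fire action calls Fire on press, with that logic defined outside these graphs.
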(event EventBeginPlay
  (Class|Tank|SetTurretReference (Variables|Default|GetTankTurret1))
  (Class|Tank|SetBarrelReference (Variables|Default|GetTankBarrel1)))

(event Input|ActionEvents|InputActionFire
  (params (Key :type Key%20Structure))
  ;[1 1 1] Input Action Binding
  (:Pressed
    (Class|Tank|Fire)))

(event Input|AxisEvents|InputAxisAimHorizontal
  (params (AxisValue :type Float%20%28single-precision%29))
  ;[1 1 1] Camera Input Binding
  (Transformation|AddRelativeRotation (Variables|Default|GetSpringArm) (Math|Rotator|MakeRotator 0.0 0.0 (* AxisValue (Utilities|Time|GetWorldDeltaSeconds) 1e+02)) false false))

(event Input|AxisEvents|InputAxisAimVertical
  (params (AxisValue :type Float%20%28single-precision%29))
  ;[1 1 1] Camera Input Binding
  (Transformation|AddRelativeRotation (Variables|Default|GetElevation%20Gimbal) (Math|Rotator|MakeRotator 0.0 AxisValue 0.0) false false))

(fn ConstructionScript)